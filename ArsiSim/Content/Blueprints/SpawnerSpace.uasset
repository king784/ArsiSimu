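; Spawner that periodically creates Enemy2 AI at random points inside its Box volume.
; After a startup delay it caches the PlayerChar, which also holds back spawning until then.
; Tick runs through a Delay to attempt a spawn about once a second.
; Each attempt requires CanSpawn, an Enemy2 count not above MaxEnemies, and the player's MustaAukko flag to be off.
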(event Custom|Spawn%20Enemy
  (bind _box (Variables|Default|GetBox))
  (if (Variables|Default|GetcanSpawn)
    (bind _outactors (Actor|GetAllActorsOfClass "/Game/Blueprints/Enemy2.Enemy2_C"))
    (if (>= (Variables|Default|GetmaxEnemies) (Utilities|Array|Length _outactors))
      (if (Utilities|IsValid (stale EventBeginPlay _asplayer_char))
        (if (not (Variables|/Game/Blueprints/PlayerChar.PlayerChar_C|GetMustaAukko (stale EventBeginPlay _asplayer_char)))
          (AI|SpawnAIFromClass "/Game/Blueprints/Enemy2.Enemy2_C" 0 (Math|Random|RandomPointinBoundingBox (Transformation|GetWorldLocation _box) (Components|Box|GetScaledBoxExtent _box)) "0, 0, 0" false))))))

(event EventTick
  (params (DeltaSeconds :type Float%20%28single-precision%29))
  (Utilities|FlowControl|Delay 1.0)
  (CallFunction|SpawnEnemy))

(event EventBeginPlay
  (Utilities|FlowControl|Delay 9.0)
  (bind _asplayer_char (Utilities|Casting|CastToPlayerChar (Game|Player|GetPlayerPawn 0))))

(fn ConstructionScript)