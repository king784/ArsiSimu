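; Spawner Blueprint that spawns Enemy2 AI pawns at random points inside its Box volume.
; Tick runs a Delay as a repeating timer, much shorter in the StadionEndless level than in other levels.
; Each spawn requires the live Enemy2 count to be within MaxEnemies and the player's MustaAukko flag to be off.
; After spawning, MaxEnemies becomes the player's Score plus one, so the cap follows score.
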(event Custom|Spawn%20Enemy
  (bind _box (Variables|Default|GetBox))
  (bind _outactors (Actor|GetAllActorsOfClass "/Game/Blueprints/Enemy2.Enemy2_C"))
  (if (>= (Variables|Default|GetmaxEnemies) (Utilities|Array|Length _outactors))
    (if (not (Variables|/Game/Blueprints/PlayerChar.PlayerChar_C|GetMustaAukko (stale EventBeginPlay _asplayer_char)))
      (AI|SpawnAIFromClass "/Game/Blueprints/Enemy2.Enemy2_C" 0 (Math|Random|RandomPointinBoundingBox (Transformation|GetWorldLocation _box) (Components|Box|GetScaledBoxExtent _box)) "0, 0, 0" false)
      (Variables|Default|SetmaxEnemies (+ (Variables|/Game/Blueprints/PlayerChar.PlayerChar_C|Getscore (stale EventBeginPlay _asplayer_char)) 1)))))

(event EventTick
  (params (DeltaSeconds :type Float%20%28single-precision%29))
  (if (Utilities|Enum|Equal(Enum) (stale EventBeginPlay _returnvalue) "StadionEndless")
    (Utilities|FlowControl|Delay 0.3)
    (CallFunction|SpawnEnemy)
    (else
      (Utilities|FlowControl|Delay 3.0)
      (CallFunction|SpawnEnemy))))

(event EventBeginPlay
  (bind _returnvalue (Game|GetCurrentLevelName true))
  (bind _asplayer_char (Utilities|Casting|CastToPlayerChar (Game|Player|GetPlayerPawn 0))))

(fn ConstructionScript)