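; Thrown shot ("kuula") that launches along the player's facing with their charged power and takes steering forces from axis input in flight.
; Tick pulls it toward a black hole when the player flags one.
; Overlaps wake Earth physics or knock small asteroids away.
; Touching ground, or leaving the hollow sphere in the Space level, updates player state, re-enables input after a delay and destroys the ball.
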(event Collision|EventActorBeginOverlap
  (params (OtherActor :type Actor%20Object%20Reference))
  (bind _playerref (Variables|Default|GetplayerRef))
  (bind _smallasteroidref (Variables|Default|GetsmallAsteroidRef))
  (bind _staticmeshcomponent (Variables|/Script/Engine.StaticMeshActor|GetStaticMeshComponent _smallasteroidref))
  ;[1 1 1] ActorBeginOverlap
  (Utilities|IsValid OtherActor
    (:Is%20Valid
      (Utilities|FlowControl|Sequence
        (:then_0
          (if (Actor|ActorHasTag OtherActor "ground")
            (Variables|/Game/Blueprints/PlayerChar.PlayerChar_C|SetONKOKUULAMAASSSA (Variables|Default|GetplayerRef) true)
            (Variables|/Game/Blueprints/PlayerChar.PlayerChar_C|SetKuulaIlmassa _playerref false)
            (Utilities|FlowControl|Delay 2.0)
            (Input|EnableInput _playerref (Game|GetPlayerController 0))
            (Variables|/Game/Blueprints/PlayerChar.PlayerChar_C|SetcanPlayTyonnonaloitus _playerref true)
            (Variables|Default|SetkuulaElossa false)
            (Variables|/Game/Blueprints/PlayerChar.PlayerChar_C|SetcanPlayTyontofail _playerref true)
            (Variables|/Game/Blueprints/PlayerChar.PlayerChar_C|SetsaaHeittaa _playerref true)
            (Utilities|Time|ClearTimerbyFunctionName _playerref "VoimanLataus")
            (Actor|DestroyActor)))
        (:then_1
          (if (== (Utilities|GetClass OtherActor) "/Game/Blueprints/earth_bp.earth_bp_C")
            (Physics|SetSimulatePhysics (Variables|/Script/Engine.StaticMeshActor|GetStaticMeshComponent (Variables|Default|GetearthRef)) true)))
        (:then_2
          (if (== (Utilities|GetClass OtherActor) "/Game/Blueprints/smallAsteroid_bp.smallAsteroid_bp_C")
            (Physics|SetSimulatePhysics _staticmeshcomponent true)
            (Physics|SetEnableGravity _staticmeshcomponent false)
            (Physics|AddImpulse _staticmeshcomponent (* (- (Transformation|GetActorLocation _smallasteroidref) (Transformation|GetActorLocation)) 5e+03) "None" false)))))))

(event EventBeginPlay
  (bind _returnvalue (Game|Player|GetPlayerPawn 0))
  ;[1 1 1] Alkuarvojen alustus ja alkuvoiman antaminen
  (Utilities|FlowControl|Sequence
    (:then_0
      (bind _asplayer_char (Utilities|Casting|CastToPlayerChar (Game|GetPlayerCharacter 0)))
      (Variables|Default|SetplayerRef _asplayer_char))
    (:then_1
      (Variables|Default|SetkuulaElossa true)
      (Variables|/Game/Blueprints/PlayerChar.PlayerChar_C|SetrotationLock (Variables|Default|GetplayerRef) false)
      (Variables|/Game/Blueprints/PlayerChar.PlayerChar_C|SetisTyonto (Variables|Default|GetplayerRef) false)
      (Variables|/Game/Blueprints/PlayerChar.PlayerChar_C|SetMaksalaatikko (Variables|Default|GetplayerRef) false)
      (Variables|/Game/Blueprints/PlayerChar.PlayerChar_C|SetONKOKUULAMAASSSA (Variables|Default|GetplayerRef) false)
      (Variables|/Game/Blueprints/PlayerChar.PlayerChar_C|SetKuulaIlmassa (Variables|Default|GetplayerRef) true)
      (Utilities|FlowControl|Sequence
        (:then_0
          (bind _outactors (Actor|GetAllActorsOfClass "/Script/Landscape.Landscape"))
          (for _array_element _outactors
            (Variables|Default|SetlandscapeRef _array_element))
          (Input|EnableInput (Game|GetPlayerController 0))
          (bind _asplayer_char_2 (Utilities|Casting|CastToPlayerChar _returnvalue))
          (Physics|AddImpulse (Variables|Default|GetSphere) (* (Math|Vector|GetForwardVector (Transformation|GetActorRotation _returnvalue)) (Variables|/Game/Blueprints/PlayerChar.PlayerChar_C|GetVoima _asplayer_char_2)) "None" false))
        (:then_1
          (bind _outactors_2 (Actor|GetAllActorsOfClass "/Game/Blueprints/earth_bp.earth_bp_C"))
          (for _array_element_2 _outactors_2
            (Variables|Default|SetearthRef _array_element_2)))
        (:then_2
          (bind _returnvalue_2 (Game|GetCurrentLevelName true))
          (if (Utilities|Enum|Equal(Enum) _returnvalue_2 "Space")
            (Variables|Default|SetisHollowWorld true)
            (bind _outactors_3 (Actor|GetAllActorsOfClass "/Game/Blueprints/hollowSphere_bp.hollowSphere_bp_C"))
            (for _array_element_3 _outactors_3
              (Variables|Default|SethollowSphereRef _array_element_3))))
        (:then_3
          (bind _outactors_4 (Actor|GetAllActorsOfClass "/Game/Blueprints/smallAsteroid_bp.smallAsteroid_bp_C"))
          (for _array_element_4 _outactors_4
            (Variables|Default|SetsmallAsteroidRef _array_element_4)))))))

(event EventTick
  (params (DeltaSeconds :type Float%20%28single-precision%29))
  (bind _playerref (Variables|Default|GetplayerRef))
  (bind _playerref_2 (Variables|Default|GetplayerRef))
  ;[1 1 1] Event Tick/Kuula kohti mustaa aukkoa
  (Utilities|FlowControl|Sequence
    (:then_0
      (if (Variables|/Game/Blueprints/PlayerChar.PlayerChar_C|Getmustaaukko _playerref)
        (Utilities|FlowControl|Delay 0.1)
        (if true
          (Physics|AddImpulse (Variables|Default|GetSphere) (* (- (Variables|/Game/Blueprints/PlayerChar.PlayerChar_C|GetMustaAukkoLocation _playerref) (Transformation|GetActorLocation)) 4.5) "None" false))))
    (:then_1
      (Utilities|FlowControl|Delay 0.1)
      (if (Variables|Default|GetisHollowWorld)
        (if (not (Collision|IsOverlappingActor (Variables|Default|GethollowSphereRef) :!class /Script/Engine.Actor))
          (Variables|/Game/Blueprints/PlayerChar.PlayerChar_C|SetONKOKUULAMAASSSA _playerref_2 true)
          (Variables|/Game/Blueprints/PlayerChar.PlayerChar_C|SetKuulaIlmassa _playerref_2 false)
          (Utilities|FlowControl|Delay 2.0)
          (Input|EnableInput _playerref_2 (Game|GetPlayerController 0))
          (Variables|Default|SetkuulaElossa false)
          (Actor|DestroyActor))))))

(event Collision|EventActorEndOverlap
  (params (OtherActor :type Actor%20Object%20Reference))
  (bind _returnvalue (Game|GetPlayerController 0))
  (bind _playerref (Variables|Default|GetplayerRef))
  ;[1 1 1] ActorEndOverlap
  (if (Variables|Default|GetisHollowWorld)
    (if (== (Utilities|GetClass OtherActor) "/Game/Blueprints/hollowSphere_bp.hollowSphere_bp_C")
      (Variables|/Game/Blueprints/PlayerChar.PlayerChar_C|SetONKOKUULAMAASSSA _playerref true)
      (Variables|/Game/Blueprints/PlayerChar.PlayerChar_C|SetKuulaIlmassa _playerref false)
      (Utilities|FlowControl|Delay 2.0)
      (Input|EnableInput _playerref _returnvalue)
      (Variables|/Game/Blueprints/PlayerChar.PlayerChar_C|SetcanPlayTyonnonaloitus _playerref true)
      (Variables|Default|SetkuulaElossa false)
      (Variables|/Game/Blueprints/PlayerChar.PlayerChar_C|SetcanPlayTyontofail _playerref true)
      (Variables|/Game/Blueprints/PlayerChar.PlayerChar_C|SetsaaHeittaa _playerref true)
      (Utilities|Time|ClearTimerbyFunctionName _returnvalue "VoimanLataus")
      (Actor|DestroyActor))))

(event Input|AxisEvents|InputAxisRight
  (params (AxisValue :type Float%20%28single-precision%29))
  ;[1 1 1] Kuulan liikutus vasemmalle/oikealle ilmassa
  (Physics|AddForce (Variables|Default|GetSphere) (Math|Transform|TransformDirection (Transformation|GetActorTransform (Game|GetPlayerCharacter 0)) (Math|Vector|MakeVector 0.0 (* AxisValue 1e+05) 0.0)) "None" false))

(event Input|AxisEvents|InputAxisUp
  (params (AxisValue :type Float%20%28single-precision%29))
  (bind _sphere (Variables|Default|GetSphere))
  ;[1 1 1] Kuulan liikutus eteen/taakse ilmassa
  (Utilities|IsValid _sphere
    (:Is%20Valid
      (Physics|AddForce _sphere (* (* (Math|Vector|GetForwardVector (Variables|/Script/Engine.Character|GetCapsuleComponent (Game|GetPlayerCharacter 0))) "0,1.000000, 0") (* AxisValue 7e+04)) "None" false))))

(fn ConstructionScript)