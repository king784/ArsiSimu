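; Maksalaatikko is a spinning pickup actor that flags the player character as having collected it.
; In the "Space" level, BeginPlay shows its cylinder mesh and limits it to a short lifespan.
; An overlap with an actor tagged "kuula" plays the Pling sound, sets the Maksalaatikko flag on the player's PlayerChar pawn and destroys the pickup.
; Tick adds a constant world rotation each frame, independent of delta time.
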(event Collision|EventActorBeginOverlap
  (params (OtherActor :type Actor%20Object%20Reference))
  (if (Actor|ActorHasTag OtherActor "kuula")
    (Audio|Components|Audio|Play (Variables|Default|GetPling) 0.0)
    (bind _asplayer_char (Utilities|Casting|CastToPlayerChar (Game|Player|GetPlayerPawn 0)))
    (Variables|/Game/Blueprints/PlayerChar.PlayerChar_C|SetMaksalaatikko _asplayer_char true)
    (Actor|DestroyActor)))

(event EventTick
  (params (DeltaSeconds :type Float%20%28single-precision%29))
  (Class|Actor|AddActorWorldRotation "0.000000,1.000000,0.000000"))

(event EventBeginPlay
  (bind _returnvalue (Game|GetCurrentLevelName true))
  (if (Utilities|Enum|Equal(Enum) _returnvalue "Space")
    (Rendering|SetVisibility (Variables|Default|GetCylinder) true false)
    (Actor|SetLifeSpan 15.0)))

(fn ConstructionScript)