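; Level 2 enemy spawner actor that keeps Enemy2 AI pawns populated inside a box volume.
; Every tick it counts all Enemy2 actors in the world and, while four or fewer exist, spawns another at a random point within its Box component's bounds.
; An unconnected leftover lookup of a random Spawner_lvl2 instance never runs.
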(event EventBeginPlay)

(event Collision|EventActorBeginOverlap
  (params (OtherActor :type Actor%20Object%20Reference)))

(event EventTick
  (params (DeltaSeconds :type Float%20%28single-precision%29))
  (bind _box (Variables|Default|GetBox))
  (bind _outactors (Actor|GetAllActorsOfClass "/Game/Blueprints/Enemy2.Enemy2_C"))
  (if (>= 4 (Utilities|Array|Length _outactors))
    (AI|SpawnAIFromClass "/Game/Blueprints/Enemy2.Enemy2_C" 0 (Math|Random|RandomPointinBoundingBox (Transformation|GetWorldLocation _box) (Components|Box|GetScaledBoxExtent _box)) "0, 0, 0" false)))

(fn ConstructionScript)