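; Spawner Blueprint that places Maksalaatikko actors at a randomly picked MaksaLaatikkoSpawn point, chosen from the first three found.
; Tick, throttled by a Delay, spawns when it is not overlapping MaksalaatikkoRef, CanSpawn is true and the Laatikot count is within MaxLaatikot.
; Each spawn clears CanSpawn, which this graph never re-enables, increments Laatikot and starts a one-shot timer that later decrements the count.
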(event Custom|vahemmanLaatikoita
  (bind _result (Math|Integer|DecrementInt (Variables|Default|Getlaatikot))
    (:%20%20
      (Variables|Default|Setlaatikot _result))))

(event EventTick
  (params (DeltaSeconds :type Float%20%28single-precision%29))
  (Utilities|FlowControl|Delay 0.2)
  (if (not (Collision|IsOverlappingActor (Variables|Default|GetmaksalaatikkoRef) :!class /Script/Engine.Actor))
    (if (Variables|Default|GetcanSpawn)
      (if (<= (Variables|Default|Getlaatikot) (Variables|Default|GetmaxLaatikot))
        (Variables|Default|SetcanSpawn false)
        (bind _outactors (Actor|GetAllActorsOfClass "/Game/Blueprints/MaksaLaatikkoSpawn.MaksaLaatikkoSpawn_C"))
        (Game|SpawnActorfromClass "/Game/Blueprints/Maksalaatikko.Maksalaatikko_C" (Math|Transform|MakeTransform (Transformation|GetActorLocation (Utilities|Array|Get(acopy) _outactors (Math|Random|RandomIntegerinRange 0 2))) "0, 0, 0" "1,1,1") "Undefined" 0 0)
        (bind _result (Math|Integer|IncrementInt (Variables|Default|Getlaatikot))
          (:%20%20
            (Variables|Default|Setlaatikot _result)
            (Utilities|Time|SetTimerbyEvent (delegate Custom|vahemmanLaatikoita) 15.0)))))))

(fn ConstructionScript)