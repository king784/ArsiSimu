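; Projectile Blueprint, apparently a ball, launched with a strength taken from the player character.
; On BeginPlay it enables player input, casts the player pawn to PlayerChar and sets the projectile movement's local-space velocity to the pawn's forward vector scaled by its Voima value.
; The Right input axis event is empty, with a leftover unconnected vector calculation.
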(event EventBeginPlay
  (bind _returnvalue (Game|Player|GetPlayerPawn 0))
  (Input|EnableInput (Game|GetPlayerController 0))
  (bind _asplayer_char (Utilities|Casting|CastToPlayerChar _returnvalue))
  (Game|Components|ProjectileMovement|SetVelocityinLocalSpace (Variables|Default|GetProjectileMovement) (* (Math|Vector|GetForwardVector (Transformation|GetActorRotation _returnvalue)) (Variables|/Game/Blueprints/PlayerChar.PlayerChar_C|GetVoima _asplayer_char))))

(event Input|AxisEvents|InputAxisRight
  (params (AxisValue :type Float%20%28single-precision%29)))

(fn ConstructionScript)