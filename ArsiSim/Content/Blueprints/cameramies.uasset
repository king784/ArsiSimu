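; Camera-rig actor, judging by its name, that follows the player's Kuula actor while facing the same way as the player.
; BeginPlay caches the player pawn as PlayerChar.
; Each Tick moves the root to KuulaRef's location plus a fixed world-space offset, behind on X and below, without sweeping.
; It also sets the root's yaw from the player pawn, so the offset itself does not rotate.
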(event EventBeginPlay
  (bind _asplayer_char (Utilities|Casting|CastToPlayerChar (Game|Player|GetPlayerPawn 0))))

(event EventTick
  (params (DeltaSeconds :type Float%20%28single-precision%29))
  (bind _defaultsceneroot (Variables|Default|GetDefaultSceneRoot))
  (Transformation|SetWorldLocation _defaultsceneroot (+ (Transformation|GetActorLocation (Variables|/Game/Blueprints/PlayerChar.PlayerChar_C|GetkuulaRef (stale EventBeginPlay _asplayer_char))) "-50.000000,0.000000,-50.000000") false false)
  (Transformation|SetWorldRotation _defaultsceneroot (Math|Rotator|MakeRotator 0.0 0.0 (.yaw (Transformation|GetActorRotation (Game|Player|GetPlayerPawn 0)))) false false))

(fn ConstructionScript)