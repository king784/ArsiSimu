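; Audio manager Blueprint that prepares level-specific sound, assigning an applause clip when the current level is the Stadion stage.
; On BeginPlay it caches the player character reference, then checks the level name to set the sound on its audio component.
; A playSound event plays that audio component from the start when triggered.
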(event Custom|playSound
  ;[1 1 1] playSound
  (Audio|Components|Audio|Play (Variables|Default|GetAudio) 0.0))

(event EventBeginPlay
  (Utilities|FlowControl|Sequence
    (:then_0
      (bind _asplayer_char (Utilities|Casting|CastToPlayerChar (Game|GetPlayerCharacter 0)))
      (Variables|Default|SetplayerRef _asplayer_char))
    (:then_1
      (bind _returnvalue (Game|GetCurrentLevelName true))
      (if (Utilities|Enum|Equal(Enum) _returnvalue "Stadion")
        (Audio|Components|Audio|SetSound (Variables|Default|GetAudio) "/Game/Sounds/252913__psyche-sound-studios__applause-medium_short.252913__psyche-sound-studios__applause-medium_short")))))

(fn ConstructionScript)