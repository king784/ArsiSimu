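; FalseHarju is a flying boss that faces the player, shuttles between start and end points, and pulls the player's Kuula toward its black hole.
; Overlapping the Kuula stuns it and costs HP, exploding it at zero or darkening its materials, dropping it, disabling collision and enabling two spawners.
; Chained timelines handle flight, descent and, after a delay, recovery to the start point, where only the SpawnerSpace spawner is switched off again.
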(event OnComponentBeginOverlap(FalseHarjuMesh)
  (params (OverlappedComponent :type Primitive%20Component%20Object%20Reference) (OtherActor :type Actor%20Object%20Reference) (OtherComp :type Primitive%20Component%20Object%20Reference) (OtherBodyIndex :type Integer) (bFromSweep :type Boolean) (SweepResult :type Hit%20Result%20Structure%20%28by%20ref%29))
  (if (Utilities|IsValid (Variables|Default|GetplayerRef))
    (if false
      (Variables|Default|Setstunned true))))

(event EventBeginPlay
  (bind _returnvalue (Transformation|GetActorLocation))
  (bind _returnvalue_2 (Transformation|GetActorLocation))
  (bind _falsefly (Variables|Default|GetFalseFly))
  (bind _falsefly_2 (Variables|Default|GetFalseFly))
  (Utilities|FlowControl|Delay 6.0)
  (Utilities|FlowControl|Sequence
    (:then_0
      (bind _outactors (Actor|GetAllActorsOfClass "/Game/Blueprints/StartPoint_bp.StartPoint_bp_C"))
      (for _array_element _outactors
        (Variables|Default|SetstartPointRef _array_element)))
    (:then_1
      (bind _outactors_2 (Actor|GetAllActorsOfClass "/Game/Blueprints/EndPoint_bp.EndPoint_bp_C"))
      (for _array_element_2 _outactors_2
        (Variables|Default|SetendPointRef _array_element_2)))
    (:then_2
      (Transformation|SetActorLocation (Transformation|GetActorLocation (Variables|Default|GetstartPointRef)) false false))
    (:then_3
      (bind _outactors_3 (Actor|GetAllActorsOfClass "/Game/Blueprints/PlayerChar.PlayerChar_C"))
      (for _array_element_3 _outactors_3
        (Variables|Default|SetplayerRef _array_element_3)))
    (:then_4
      (bind _outactors_4 (Actor|GetAllActorsOfClass "/Game/Blueprints/SpawnerSpace.SpawnerSpace_C"))
      (for _array_element_4 _outactors_4
        (Variables|Default|SetSpawnerRef _array_element_4)))
    (:then_5
      (bind _outactors_5 (Actor|GetAllActorsOfClass "/Game/Blueprints/MaksalaatikkoSpawner.MaksalaatikkoSpawner_C"))
      (for _array_element_5 _outactors_5
        (Variables|Default|SetmaksaLaatikkoSpawnerRef _array_element_5)))
    (:then_6
      (bind _alpha (Timeline|Flying Play)
        (:Update
          (Utilities|FlowControl|Sequence
            (:then_0
              (Utilities|IsValid (Variables|/Game/Blueprints/PlayerChar.PlayerChar_C|GetkuulaRef (Variables|Default|GetplayerRef))
                (:Is%20Valid
                  (Physics|AddImpulse (Variables|/Game/Blueprints/kuula4.kuula4_C|GetSphere (Variables|/Game/Blueprints/PlayerChar.PlayerChar_C|GetkuulaRef (Variables|Default|GetplayerRef))) (* (- (Transformation|GetWorldLocation (Variables|Default|GetBlackHole)) (Transformation|GetActorLocation (Variables|/Game/Blueprints/PlayerChar.PlayerChar_C|GetkuulaRef (Variables|Default|GetplayerRef)))) 0.5) "None" false))))
            (:then_1
              _))
          (if (Variables|Default|Getstunned)
            (Variables|Default|SetdownEndPoint (- _returnvalue_2 "0, 0,15.000000") :!label _label)
            (Variables|/Game/Blueprints/SpawnerSpace.SpawnerSpace_C|SetcanSpawn (Variables|Default|GetSpawnerRef) true)
            (Variables|/Game/Blueprints/MaksalaatikkoSpawner.MaksalaatikkoSpawner_C|SetcanSpawn (Variables|Default|GetmaksaLaatikkoSpawnerRef) true)
            (Rendering|SetVisibility (Variables|Default|GetBlackHole) false false)
            (if (Variables|Default|GetcanDamage)
              (Variables|Default|SetcanDamage false)
              (bind _result (Math|Integer|DecrementInt (Variables|Default|GetHP))
                (:%20%20
                  (Variables|Default|SetHP _result)
                  (if (<= (Variables|Default|GetHP) 0)
                    (Effects|SpawnEmitteratLocation "/Game/StarterContent/Particles/P_Explosion.P_Explosion" (Transformation|GetActorLocation))
                    (Actor|DestroyActor)
                    (else
                      (Rendering|Material|SetMaterial _falsefly_2 0 "/Game/FalseSettii/FalseBlackHole_mat.FalseBlackHole_mat")
                      (Rendering|Material|SetMaterial _falsefly_2 1 "/Game/FalseSettii/FalseBlackHole_mat.FalseBlackHole_mat")
                      (Rendering|Material|SetMaterial _falsefly_2 2 "/Game/FalseSettii/FalseBlackHole_mat.FalseBlackHole_mat")
                      (Rendering|Material|SetMaterial _falsefly_2 3 "/Game/FalseSettii/FalseBlackHole_mat.FalseBlackHole_mat")
                      (Rendering|Material|SetMaterial _falsefly_2 4 "/Game/FalseSettii/FalseBlackHole_mat.FalseBlackHole_mat")
                      (Rendering|Material|SetMaterial _falsefly_2 5 "/Game/FalseSettii/FalseBlackHole_mat.FalseBlackHole_mat")
                      (Collision|SetActorEnableCollision false)
                      (bind _alpha_2 (Timeline|DownAndUp PlayFromStart)
                        (:Update
                          (Transformation|SetActorLocation (Math|Vector|Lerp(Vector) _returnvalue_2 (Variables|Default|GetdownEndPoint) _alpha_2) false false))
                        (:Finished
                          (if (Variables|Default|Getstunned)
                            (Utilities|FlowControl|Delay 15.0)
                            (Variables|Default|Setstunned false)
                            (Timeline|DownAndUp Reverse)
                            (else
                              (Variables|Default|SetcanDamage true)
                              ;[1 1 1] SpawnerSpace canspawn
                              (Variables|/Game/Blueprints/SpawnerSpace.SpawnerSpace_C|SetcanSpawn (Variables|Default|GetSpawnerRef) false)
                              (Rendering|SetVisibility (Variables|Default|GetBlackHole) true false)
                              (if (<= (Math|Vector|VectorLength (- _returnvalue (Transformation|GetActorLocation (Variables|Default|GetstartPointRef)))) (Math|Vector|VectorLength (- _returnvalue (Transformation|GetActorLocation (Variables|Default|GetendPointRef)))))
                                (Variables|Default|SetnewEndPoint (Transformation|GetActorLocation (Variables|Default|GetstartPointRef)))
                                (else
                                  (Variables|Default|SetnewEndPoint (Transformation|GetActorLocation (Variables|Default|GetstartPointRef)))))
                              (Audio|PlaySound2D "/Game/Sounds/arsiWavit/falseharjunauru.falseharjunauru")
                              (bind _alpha_3 (Timeline|BackToPoint PlayFromStart)
                                (:Update
                                  (Transformation|SetActorLocation (Math|Vector|Lerp(Vector) _returnvalue (Variables|Default|GetnewEndPoint) _alpha_3) false false))
                                (:Finished
                                  (Rendering|Material|SetMaterial _falsefly 0 "/Game/FalseSettii/FalseSimmutJee.FalseSimmutJee")
                                  (Rendering|Material|SetMaterial _falsefly 1 "/Game/FalseSettii/FalseIho_Mat.FalseIho_Mat")
                                  (Rendering|Material|SetMaterial _falsefly 2 "/Game/FalseSettii/FalseHuivi_Mat.FalseHuivi_Mat")
                                  (Rendering|Material|SetMaterial _falsefly 3 "/Game/FalseSettii/FalseParta_Mat.FalseParta_Mat")
                                  (Rendering|Material|SetMaterial _falsefly 4 "/Game/FalseSettii/FalseBody.FalseBody")
                                  (Rendering|Material|SetMaterial _falsefly 5 "/Game/FalseSettii/FalseKengat.FalseKengat")
                                  (Collision|SetActorEnableCollision true)
                                  (Timeline|Flying PlayFromStart))))))))))))
            (elif (Collision|IsOverlappingActor (Variables|/Game/Blueprints/PlayerChar.PlayerChar_C|GetkuulaRef (Variables|Default|GetplayerRef)) :!class /Script/Engine.Actor)
              (Variables|Default|Setstunned true)
              (else
                (Transformation|SetActorLocation (Math|Vector|Lerp(Vector) (Transformation|GetActorLocation (Variables|Default|GetstartPointRef)) (Transformation|GetActorLocation (Variables|Default|GetendPointRef)) _alpha) false false)))))
        (:Finished
          (if (Variables|Default|Getstunned)
            (goto _label)
            (elif (Variables|Default|GetletsLoop)
              (Variables|Default|SetletsLoop false)
              (Timeline|Flying ReverseFromEnd)
              (else
                (Variables|Default|SetletsLoop true)
                (Timeline|Flying PlayFromStart)))))))))

(event EventTick
  (params (DeltaSeconds :type Float%20%28single-precision%29))
  (bind _playerref (Variables|Default|GetplayerRef))
  (if (Utilities|IsValid _playerref)
    (Transformation|SetActorRotation (Math|Rotator|FindLookatRotation (Transformation|GetActorLocation) (Transformation|GetActorLocation _playerref)))))

(fn ConstructionScript)