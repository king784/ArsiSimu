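; Zombie enemy actor that moans at random intervals and ends the game when it touches the player.
; A hit from a "kuula" ball launches the ball, adds score, plays impact audio through the player and AudioManager, then destroys the enemy.
; Each moan re-arms its timer with a new random delay via a Tick-checked flag.
; Tick also destroys the enemy while the player's MustaAukko (black hole) flag is set.
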(event Custom|playMoan
  (bind _audio (Variables|Default|GetAudio))
  (switch int (Math|Random|RandomIntegerinRange 0 7)
    (:0
      (Audio|Components|Audio|SetSound _audio "/Game/Sounds/arsiWavit/zombiaania/zombi1.zombi1"))
    (:1
      (Audio|Components|Audio|SetSound _audio "/Game/Sounds/arsiWavit/zombiaania/zombi2.zombi2"))
    (:2
      (Audio|Components|Audio|SetSound _audio "/Game/Sounds/arsiWavit/zombiaania/zombi3.zombi3"))
    (:3
      (Audio|Components|Audio|SetSound _audio "/Game/Sounds/arsiWavit/zombiaania/zombi4.zombi4"))
    (:4
      (Audio|Components|Audio|SetSound _audio "/Game/Sounds/arsiWavit/zombiaania/zombi5.zombi5"))
    (:5
      (Audio|Components|Audio|SetSound _audio "/Game/Sounds/arsiWavit/zombiaania/zombi6.zombi6"))
    (:6
      (Audio|Components|Audio|SetSound _audio "/Game/Sounds/arsiWavit/zombiaania/zombi7.zombi7"))
    (:7
      (Audio|Components|Audio|SetSound _audio "/Game/Sounds/arsiWavit/zombiaania/zombi8.zombi8")))
  (Audio|Components|Audio|Play _audio 0.0)
  (Variables|Default|SetcanPlaySound true))

(event Custom|playBlam
  (bind _blam (Variables|Default|GetBlam))
  ;[1 1 1] playBlam
  (Utilities|IsValid _blam
    (:Is%20Valid
      (switch int (Math|Random|RandomIntegerinRange 0 4)
        (:0
          (Audio|Components|Audio|SetSound _blam "/Game/Sounds/arsiWavit/lossahduksia/losahus1.losahus1")
          (Audio|Components|Audio|Play _blam 0.0 :!label _label))
        (:1
          (Audio|Components|Audio|SetSound _blam "/Game/Sounds/arsiWavit/lossahduksia/losahus2.losahus2")
          (goto _label))
        (:2
          (Audio|Components|Audio|SetSound _blam "/Game/Sounds/arsiWavit/lossahduksia/losahus3.losahus3")
          (goto _label))
        (:3
          (Audio|Components|Audio|SetSound _blam "/Game/Sounds/arsiWavit/lossahduksia/losahus4.losahus4"))
        (:4
          (Audio|Components|Audio|SetSound _blam "/Game/Sounds/arsiWavit/plats.plats"))))))

(event EventBeginPlay
  ;[1 1 1] BeginPlay/Event Tick/Tuhoutuminen mustasta aukosta
  (Utilities|FlowControl|Sequence
    (:then_0
      (bind _asplayer_char (Utilities|Casting|CastToPlayerChar (Game|Player|GetPlayerPawn 0))))
    (:then_1
      (bind _outactors (Actor|GetAllActorsOfClass "/Game/Blueprints/AudioManager_bp.AudioManager_bp_C"))
      (for _array_element _outactors
        (Variables|Default|SetaudioManagerRef _array_element)))
    (:then_2
      (Variables|Default|SetcanPlaySound true))))

(event EventTick
  (params (DeltaSeconds :type Float%20%28single-precision%29))
  ;[1 1 1] BeginPlay/Event Tick/Tuhoutuminen mustasta aukosta
  (Utilities|FlowControl|Sequence
    (:then_0
      (if (Utilities|IsValid (stale EventBeginPlay _asplayer_char))
        (if (Variables|/Game/Blueprints/PlayerChar.PlayerChar_C|GetMustaAukko (stale EventBeginPlay _asplayer_char))
          (Actor|DestroyActor))))
    (:then_1
      (if (Variables|Default|GetcanPlaySound)
        (Utilities|Time|SetTimerbyEvent (delegate Custom|playMoan) (Math|Random|RandomFloatinRange 3.0 6.0) true)
        (Variables|Default|SetcanPlaySound false)))))

(event Collision|EventActorBeginOverlap
  (params (OtherActor :type Actor%20Object%20Reference))
  (bind _returnvalue (Game|GetPlayerController 0))
  (bind _audiomanagerref (Variables|Default|GetaudioManagerRef))
  ;[1 1 1] ActorBeginOverlap/Score
  (Utilities|FlowControl|Sequence
    (:then_0
      (if (Actor|ActorHasTag OtherActor "kuula")
        (bind _askuula_4 (Utilities|Casting|CastTokuula4 OtherActor))
        (Physics|AddImpulse (Variables|/Game/Blueprints/kuula4.kuula4_C|GetSphere _askuula_4) "-1000.000000, 0,50000.000000" "None" false)
        (bind _asplayer_char (Utilities|Casting|CastToPlayerChar (Game|Player|GetPlayerPawn 0)))
        (Default|PlayBlamUusi _asplayer_char)
        (Variables|/Game/Blueprints/PlayerChar.PlayerChar_C|Setscore _asplayer_char (+ (Variables|/Game/Blueprints/PlayerChar.PlayerChar_C|Getscore _asplayer_char) 1))
        (Utilities|FlowControl|Sequence
          (:then_0
            (if (Utilities|IsValid _audiomanagerref)
              (Default|PlaySound _audiomanagerref)
              (Actor|DestroyActor :!label _label)))
          (:then_2
            (goto _label)))))
    (:then_1
      (if (Actor|ActorHasTag OtherActor "pelaaja")
        (Input|DisableInput (Game|GetPlayerCharacter 0) (Game|GetPlayerController 0))
        (Viewport|RemoveAllWidgets)
        (Game|SetGamePaused true)
        (bind _returnvalue_2 (UserInterface|CreateWidget "/Game/HUD/GameOver.GameOver_C" _returnvalue))
        (UserInterface|Viewport|AddtoViewport _returnvalue_2 0)
        (Variables|/Script/Engine.PlayerController|SetbEnableClickEvents _returnvalue true)
        (Variables|/Script/Engine.PlayerController|SetbShowMouseCursor _returnvalue true)))))

(fn ConstructionScript)