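; SensEnemy is an enemy pawn that chases the player on sight and ends the run on contact.
; PawnSensing detects a PlayerChar and starts an AI MoveTo toward it.
; Overlapping a "kuula"-tagged ball (kuula4) launches that ball's sphere mostly upward with an impulse and destroys the enemy.
; Overlapping a "pelaaja"-tagged actor prints a Finnish loss message, then reloads the current level after a short delay.
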(event OnSeePawn(PawnSensing)
  (params (Pawn :type Pawn%20Object%20Reference))
  (bind _asplayer_char (Utilities|Casting|CastToPlayerChar Pawn))
  (AI|AIMoveTo self "0, 0, 0" _asplayer_char 5.0 false))

(event Collision|EventActorBeginOverlap
  (params (OtherActor :type Actor%20Object%20Reference))
  (if (Actor|ActorHasTag OtherActor "kuula")
    (bind _askuula_4 (Utilities|Casting|CastTokuula4 OtherActor))
    (Physics|AddImpulse (Variables|/Game/Blueprints/kuula4.kuula4_C|GetSphere _askuula_4) "-1000.000000, 0,75000.000000" "None" false)
    (Actor|DestroyActor)
    (elif (Actor|ActorHasTag OtherActor "pelaaja")
      (bind _returnvalue (Game|GetCurrentLevelName true))
      (Development|PrintString "HÄVISIT LOLOL")
      (Utilities|FlowControl|Delay 3.0)
      (Game|OpenLevel(byName) (Utilities|String|StringToName _returnvalue)))))

(fn ConstructionScript)