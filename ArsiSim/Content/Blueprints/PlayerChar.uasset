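; PlayerChar is a player character that aims and launches a Kuula4 ball using a hold-to-charge "tyonto" input.
; Axis inputs pitch the actor and yaw the controller.
; While held, a looping timer raises and prints Voima (force), which this graph never applies to the ball.
; Release spawns the ball at Arrow1, blends the camera view to it, then returns to the player after a delay.
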(event Custom|VoimanLataus
  (if (Variables|Default|GetisTyonto)
    (bind _output_get (Variables|Default|SetVoima (+ (Variables|Default|GetVoima) 1e+04)))
    (Development|PrintString (Utilities|String|ToString(Float) _output_get))
    (else
      (Variables|Default|SetVoima 1e+01))))

(event EventBeginPlay)

(event Collision|EventActorBeginOverlap
  (params (OtherActor :type Actor%20Object%20Reference)))

(event EventTick
  (params (DeltaSeconds :type Float%20%28single-precision%29)))

(event Input|ActionEvents|InputActiontyonto
  (params (Key :type Key%20Structure :default "AnyKey"))
  (bind _returnvalue (Game|GetPlayerController 0))
  (:Pressed
    (Variables|Default|SetisTyonto true)
    (Utilities|Time|SetTimerbyEvent (delegate Custom|VoimanLataus) 0.1 true))
  (:Released
    (bind _returnvalue_2 (Game|SpawnActorfromClass "/Game/Blueprints/kuula4.kuula4_C" (Math|Transform|MakeTransform (Transformation|GetWorldLocation (Variables|Default|GetArrow1)) "0, 0, 0" "1,1,1") "AdjustIfPossibleButAlwaysSpawn" 0 0))
    (Variables|Default|SetisTyonto false)
    (Game|Player|SetViewTargetwithBlend _returnvalue _returnvalue_2 0.0 "VTBlend_Linear" 0.0 false)
    (Utilities|FlowControl|Delay 5.0)
    (Game|Player|SetViewTargetwithBlend _returnvalue (Game|GetPlayerCharacter 0) 0.0 "VTBlend_Linear" 0.0 false)))

(event Input|AxisEvents|InputAxisUp
  (params (AxisValue :type Float%20%28single-precision%29))
  (Transformation|AddActorLocalRotation (Math|Rotator|MakeRotator 0.0 AxisValue 0.0) false false))

(event Input|AxisEvents|InputAxisRight
  (params (AxisValue :type Float%20%28single-precision%29))
  (Pawn|Input|AddControllerYawInput AxisValue))

(fn ConstructionScript)