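; Black hole actor (mustaAukko) that serves as a level exit, starting with collision disabled and writing its location to the PlayerChar.
; Tick polls the player's MustaAukko flag; while true, it shows both spheres, enables blocking collision and keeps AukkoSound playing.
; An overlap by an actor tagged "Kuula" opens Kenttä3, Space or Credits based on the player's Kentta counter, which increments for the first two.
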(event EventBeginPlay
  (Collision|SetActorEnableCollision false)
  (bind _asplayer_char (Utilities|Casting|CastToPlayerChar (Game|Player|GetPlayerPawn 0)))
  (Variables|/Game/Blueprints/PlayerChar.PlayerChar_C|SetMustaAukkoLocation _asplayer_char (Transformation|GetActorLocation)))

(event EventTick
  (params (DeltaSeconds :type Float%20%28single-precision%29))
  (if (Utilities|IsValid self)
    (if (Variables|/Game/Blueprints/PlayerChar.PlayerChar_C|GetMustaAukko (stale EventBeginPlay _asplayer_char))
      (Rendering|SetVisibility (Variables|Default|GetSphere1) true false)
      (Collision|SetActorEnableCollision true)
      (Collision|SetCollisionProfileName (Variables|Default|GetSphere) "BlockAllDynamic" :!class /Script/Engine.PrimitiveComponent)
      (if (not (Audio|Components|Audio|IsPlaying (Variables|Default|GetAukkoSound)))
        (Audio|Components|Audio|Play (Variables|Default|GetAukkoSound) 0.0)))))

(event Collision|EventActorBeginOverlap
  (params (OtherActor :type Actor%20Object%20Reference))
  (if (Actor|ActorHasTag OtherActor "Kuula")
    (switch int (Variables|/Game/Blueprints/PlayerChar.PlayerChar_C|Getkentta (stale EventBeginPlay _asplayer_char))
      (:0
        (Game|OpenLevel(byName) "Kenttä3")
        (bind _result (Math|Integer|IncrementInt (Variables|/Game/Blueprints/PlayerChar.PlayerChar_C|Getkentta (stale EventBeginPlay _asplayer_char)) :!label _label)
          (:%20%20
            (Variables|/Game/Blueprints/PlayerChar.PlayerChar_C|Setkentta (stale EventBeginPlay _asplayer_char) _result))))
      (:1
        (Game|OpenLevel(byName) "Space")
        (goto _label))
      (:2
        (Game|OpenLevel(byName) "Credits")))))

(fn ConstructionScript)